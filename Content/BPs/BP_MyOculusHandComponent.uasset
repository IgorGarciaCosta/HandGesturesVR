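; Oculus hand component that records, deletes and recognises static hand poses as named gestures.
; Recording stores every bone's component-space location in a BP_SaveGameGesture save slot, from which the gesture list loads at BeginPlay.
; A looping timer compares live bone positions to each saved gesture within a distance threshold, taking the first full match and firing OnGestureRecognised when it differs from the current one.
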(event Custom|DetectGestures
  (bind (_result _gesture) (CallFunction|GetCurrentGesture))
  (if _result
    (if (not (CallFunction|EqualGestures _gesture (Variables|Default|GetCurrentGesture)))
      (bind _output_get (Variables|Default|SetCurrentGesture _gesture))
      (Default|CallOnGestureRecognised (.GestureName (Utilities|Struct|BreakS_Gesture _output_get))))))

(event EventBeginPlay
  (Variables|Default|SetGestures (Variables|/Game/BPs/BP_SaveGameGesture.BP_SaveGameGesture_C|GetGestures (CallFunction|LoadGestures)))
  (Utilities|Time|SetTimerbyEvent (delegate Custom|DetectGestures) (Variables|Default|GetRefreshRate) true))

(event EventTick
  (params (DeltaSeconds :type Float%20%28single-precision%29)))

(fn LoadGestures
  (bind _gesturegameslot (Variables|Default|GetGestureGameSlot))
  (bind _returnvalue (SaveGame|DoesSaveGameExist _gesturegameslot))
  (if _returnvalue
    (bind _returnvalue_2 (SaveGame|LoadGamefromSlot _gesturegameslot))
    (bind _asbp_save_game_gesture (Utilities|Casting|CastToBP_SaveGameGesture _returnvalue_2))
    (return _asbp_save_game_gesture)
    (else
      (bind _returnvalue_3 (SaveGame|CreateSaveGameObject "/Game/BPs/BP_SaveGameGesture.BP_SaveGameGesture_C"))
      (return _returnvalue_3))))

(fn RecordGesture
  (params (GestureName :type String))
  (bind _output_get (LocalVariables|SetGestureSaveGame (CallFunction|LoadGestures)))
  (if (not (CallFunction|DoesGestureExist _output_get GestureName))
    (for _index (range 0 (- (Class|SkinnedMeshComponent|GetNumBones) 1))
      (bind _returnvalue (Class|PoseableMeshComponent|GetBoneLocationbyName (Class|SkinnedMeshComponent|GetBoneName _index) "ComponentSpace"))
      (Utilities|Array|Add (Variables|Default|GetBoneLocations) _returnvalue))
    (Utilities|Array|Add (Variables|/Game/BPs/BP_SaveGameGesture.BP_SaveGameGesture_C|GetGestures (LocalVariables|GetGestureSaveGame)) (Utilities|Struct|MakeS_Gesture GestureName (Variables|Default|GetBoneLocations)))
    (SaveGame|SaveGametoSlot (LocalVariables|GetGestureSaveGame) (Variables|Default|GetGestureGameSlot))))

(fn DoesGestureExist
  (params (SaveGameGesture :type BP%20Save%20Game%20Gesture%20Object%20Reference) (GestureName :type String))
  (for _array_element (Variables|/Game/BPs/BP_SaveGameGesture.BP_SaveGameGesture_C|GetGestures SaveGameGesture)
    (if (Utilities|Enum|Equal(Enum) (.GestureName (Utilities|Struct|BreakS_Gesture _array_element)) GestureName)
      (return true)))
  (return false))

(fn DeleteGesture
  (params (GestureName :type String))
  (bind _output_get (LocalVariables|SetGestureSaveGame (CallFunction|LoadGestures)))
  (for (_array_element _array_index) (Variables|/Game/BPs/BP_SaveGameGesture.BP_SaveGameGesture_C|GetGestures _output_get)
    (if (Utilities|Enum|Equal(Enum) (.GestureName (Utilities|Struct|BreakS_Gesture _array_element)) GestureName)
      (LocalVariables|SetIndex _array_index)))
  (Utilities|Array|RemoveIndex (Variables|/Game/BPs/BP_SaveGameGesture.BP_SaveGameGesture_C|GetGestures (LocalVariables|GetGestureSaveGame)) (LocalVariables|GetIndex))
  (SaveGame|SaveGametoSlot (LocalVariables|GetGestureSaveGame) (Variables|Default|GetGestureGameSlot)))

(fn GetCurrentGesture
  (for _array_element (Variables|Default|GetGestures)
    (for (_array_element_2 _array_index) (.BonesLocations (Utilities|Struct|BreakS_Gesture _array_element))
      (bind _returnvalue (Class|PoseableMeshComponent|GetBoneLocationbyName (Class|SkinnedMeshComponent|GetBoneName _array_index) "ComponentSpace"))
      (if (Variables|Default|GetDebug)
        (Development|PrintString (Utilities|String|ToString(Float) (Math|Float|Absolute(Float) (Math|Vector|VectorLength (- _returnvalue _array_element_2))))))
      (if (> (Math|Float|Absolute(Float) (Math|Vector|VectorLength (- _returnvalue _array_element_2))) (Variables|Default|GetThreshold))
        (LocalVariables|SetbValidGesture false)))
    (if (LocalVariables|GetbValidGesture)
      (return (LocalVariables|GetbValidGesture) _array_element)
      (else
        (LocalVariables|SetbValidGesture true))))
  (return false ""))

(fn EqualGestures
  (params (A :type S%20Gesture%20Structure) (B :type S%20Gesture%20Structure))
  (bind (_gesturename _boneslocations) (Utilities|Struct|BreakS_Gesture B))
  (bind (_gesturename_2 _boneslocations_2) (Utilities|Struct|BreakS_Gesture A))
  (return (and (Utilities|Enum|Equal(Enum) _gesturename_2 _gesturename) (Utilities|Array|Identical _boneslocations_2 _boneslocations))))
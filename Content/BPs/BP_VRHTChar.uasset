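; VR hand-tracking character that turns recognised hand gestures into Telegram alerts, apparently as a test setup.
; BeginPlay binds both hands' gesture events; Rock sends a help message and Point sends a fixed venue location, while OK and Hang Loose only print.
; Debug keys record gestures per hand, delete them or send a test message.
; Bot token, chat ID and venue are hardcoded, and several Telegram test calls sit unconnected.
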(event Custom|RecognizedGesture
  (params (GestureName :type String))
  (switch string GestureName
    (:Rock
      (Development|PrintString "-----------------------------------------------------ROCK")
      (Class|TelegramMessageBPLibrary|SendTelegramMessage "5246876218:AAEQ55VEJC_vYdqFHK3rgcecyZPsG1yRIAE" "1412222232" "HELP MESSAGE")
      (Development|PrintString "MESSAGE SENT"))
    (:Point
      (Development|PrintString "-----------------------------------------------------POINTER")
      (Class|TelegramMessageBPLibrary|SendTelegramVenue "5246876218:AAEQ55VEJC_vYdqFHK3rgcecyZPsG1yRIAE" "1412222232" "11.6629" "39.0085" "Serrinha" "Rua Mariano Santana")
      (Development|PrintString "LOCATION SENT"))
    (:OK
      (Development|PrintString "-----------------------------------------------------OK"))
    (:HangLoose
      (Development|PrintString "-----------------------------------------------------HANG LOOSE"))))

(event EventBeginPlay
  (EventDispatchers|BindEventtoOnGestureRecognised (Variables|Default|GetLeftHand) (EventDispatchers|CreateEvent :!event Custom|RecognizedGesture)))

(event Input|KeyboardEvents|R
  (params (Key :type Key%20Structure :default "None"))
  (:Pressed
    (Default|RecordGesture (Variables|Default|GetRightHand) (Variables|Default|GetGestureName))
    (Development|PrintString "-----------------------------------------------------RECORDED RIGHT")))

(event Input|KeyboardEvents|L
  (params (Key :type Key%20Structure :default "None"))
  (:Pressed
    (Default|RecordGesture (Variables|Default|GetLeftHand) (Variables|Default|GetGestureName))
    (Development|PrintString "-----------------------------------------------------RECORDED LEFT")))

(event Input|KeyboardEvents|D
  (params (Key :type Key%20Structure :default "None"))
  (:Pressed
    (Default|DeleteGesture (Variables|Default|GetLeftHand) (Variables|Default|GetGestureName))
    (Development|PrintString "-----------------------------------------------------DELETED GESTURE")))

(event Input|KeyboardEvents|S
  (params (Key :type Key%20Structure :default "None"))
  ;[1 1 1] Telegram functions testing
  (:Pressed
    (Class|TelegramMessageBPLibrary|SendTelegramMessage "5246876218:AAEQ55VEJC_vYdqFHK3rgcecyZPsG1yRIAE" "1412222232" "HELP MESSAGE")
    (Development|PrintString "Hello")))

(fn ConstructionScript)
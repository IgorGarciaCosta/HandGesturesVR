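; BP_VRHTChar is a character Blueprint, apparently for VR, with the beginnings of a named-gesture recording system backed by a save game.
; LoadGestures loads BP_SaveGameGesture from its slot or creates a new one, and RecordGesture passes it to DoesGestureExist.
; DoesGestureExist scans saved gestures by name but returns false on a match.
; RecordGesture ends in an empty loop without saving, and the event graph is unused.
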(event EventBeginPlay)

(event Collision|EventActorBeginOverlap
  (params (OtherActor :type Actor%20Object%20Reference)))

(event EventTick
  (params (DeltaSeconds :type Float%20%28single-precision%29)))

(fn ConstructionScript)

(fn LoadGestures
  (bind _gesturegameslot (Variables|Default|GetGestureGameSlot))
  (bind _returnvalue (SaveGame|DoesSaveGameExist _gesturegameslot))
  (if _returnvalue
    (bind _returnvalue_2 (SaveGame|LoadGamefromSlot _gesturegameslot))
    (bind _asbp_save_game_gesture (Utilities|Casting|CastToBP_SaveGameGesture _returnvalue_2))
    (return _asbp_save_game_gesture)
    (else
      (bind _returnvalue_3 (SaveGame|CreateSaveGameObject "/Game/BP_SaveGameGesture.BP_SaveGameGesture_C"))
      (return _returnvalue_3))))

(fn RecordGesture
  (params (GestureName :type String))
  (bind _output (CallFunction|LoadGestures))
  (bind _output_get (Variables|Default|SetGestureSaveGame _output))
  (bind _result (CallFunction|DoesGestureExist _output_get GestureName))
  (if (not _result)
    (for _index (range 0 0)
      _)))

(fn DoesGestureExist
  (params (SaveGameGesture :type BP%20Save%20Game%20Gesture%20Object%20Reference) (GestureName :type String))
  (for _array_element (Variables|/Game/BP_SaveGameGesture.BP_SaveGameGesture_C|GetGestures SaveGameGesture)
    (if (Utilities|Enum|Equal(Enum) (.GestureName (Utilities|Struct|BreakS_Gesture _array_element)) GestureName)
      (return false))))